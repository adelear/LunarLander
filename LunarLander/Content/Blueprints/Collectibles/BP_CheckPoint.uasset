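; BP_CheckPoint is a collectible checkpoint that counts toward the third-person character's CollectedPortals total.
; When an actor tagged Player overlaps it, it plays a sound, activates a collected effect and starts its rotating movement.
; It then increments the counter on player 0's BP_ThirdPersonCharacter and destroys itself after a short delay.
; No guard blocks repeated overlaps during that delay, so re-entering can count again.
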(event Collision|EventActorBeginOverlap
  (params (OtherActor :type Actor%20Object%20Reference))
  (if (Actor|ActorHasTag OtherActor "Player")
    (Audio|PlaySound2D "/Game/Audio/3rd-blip-95666.3rd-blip-95666" 0.5 1.0 0.0 0 0)
    (Components|Activation|Activate (Variables|Default|GetCollectedEffect) false)
    (Components|Activation|SetActive (Variables|Default|GetRotatingMovement) true false)
    (bind _asbp_third_person_character (Utilities|Casting|CastToBP_ThirdPersonCharacter (Game|GetPlayerCharacter 0)))
    (bind _result (Math|Integer|IncrementInt (Variables|/Game/Blueprints/Spaceship/BP_ThirdPersonCharacter.BP_ThirdPersonCharacter_C|GetCollectedPortals _asbp_third_person_character))
      (:%20%20
        (Variables|/Game/Blueprints/Spaceship/BP_ThirdPersonCharacter.BP_ThirdPersonCharacter_C|SetCollectedPortals _asbp_third_person_character _result)
        (Utilities|FlowControl|Delay 1.5)
        (Actor|DestroyActor)))))

(fn ConstructionScript)